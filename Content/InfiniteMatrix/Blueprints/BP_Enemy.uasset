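; BP_Enemy is an enemy actor that damages the player on contact and awards score when hit by a projectile.
; It rolls steadily every tick and reacts through its Sphere overlap.
; Player overlaps call ProcessHit, then either flag death and show restart at low health, or destroy the enemy.
; Projectile overlaps are checked a tick later, incrementing the owning player's score and destroying the enemy.
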(event OnComponentBeginOverlap(Sphere)
  (params (OverlappedComponent :type Primitive%20Component%20Object%20Reference) (OtherActor :type Actor%20Object%20Reference) (OtherComp :type Primitive%20Component%20Object%20Reference) (OtherBodyIndex :type Integer) (bFromSweep :type Boolean) (SweepResult :type Hit%20Result%20Structure%20%28by%20ref%29))
  (Utilities|FlowControl|Sequence
    (:then_0
      (bind _asbp_player (Utilities|Casting|CastToBP_Player OtherActor))
      (if (< (Variables|/Game/InfiniteMatrix/Blueprints/BP_Player.BP_Player_C|GetPlayerHealth _asbp_player) 15)
        (Default|ProcessHit _asbp_player)
        (Variables|/Game/InfiniteMatrix/Blueprints/BP_Player.BP_Player_C|SetisDead _asbp_player true)
        (Default|DisplayRestart _asbp_player)
        (else
          (Default|ProcessHit _asbp_player)
          (Actor|DestroyActor))))
    (:then_1
      (Utilities|FlowControl|DelayUntilNextTick)
      (bind _asbp_projectile (Utilities|Casting|CastToBP_Projectile OtherActor))
      (Default|IncrementScoreUp (Variables|/Game/InfiniteMatrix/Blueprints/BP_Projectile.BP_Projectile_C|GetPlayerOwner _asbp_projectile))
      (Actor|DestroyActor))))

(event EventBeginPlay)

(event Collision|EventActorBeginOverlap
  (params (OtherActor :type Actor%20Object%20Reference)))

(event EventTick
  (params (DeltaSeconds :type Float%20%28single-precision%29))
  (Transformation|AddActorLocalRotation (Math|Rotator|MakeRotator (* DeltaSeconds 5e+01) 0.0 0.0) false false))

(fn ConstructionScript)